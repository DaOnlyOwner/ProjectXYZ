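; TestDummy is an enemy test target that prints the damage it receives instead of applying it.
; ReceiveDamage passes the hit's elements and raw damage to CalculateFinalDamage, prints the result on screen for a long duration and returns true.
; Its per-element damage function scales raw damage by the square root of the element count, ignoring the element ID.
; KnockDown, Push and Shock are stubs returning false.
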(event EventBeginPlay)

(event Collision|EventActorBeginOverlap
  (params (OtherActor :type Actor%20Object%20Reference)))

(event EventTick
  (params (DeltaSeconds :type Float%20%28single-precision%29)))

(fn ConstructionScript)

(fn CalculateDamageforElementID
  (params (id :type ElementID%20Enum :default "Shield") (count :type Integer) (rawDamage :type Integer))
  (bind _returnvalue (Math|Conversions|ToFloat(Integer) count))
  (bind _returnvalue_2 (Math|Conversions|ToFloat(Integer) rawDamage))
  (bind _returnvalue_3 (|((sqrt(x))*y) _returnvalue _returnvalue_2))
  (Development|PrintString (Utilities|String|ToString(Float) _returnvalue_3) true true "(R=0.000000,G=0.660000,B=1.000000,A=1.000000)" 0.0)
  (return _returnvalue_3))

(fn KnockDown
  (return false))

(fn Push
  (params (direction :type Vector%20%28by%20ref%29 :default "0, 0, 0"))
  (return false))

(fn ReceiveDamage
  (params (damageInformation :type Damage%20Information%20Structure%20%28by%20ref%29))
  (bind (_causer _elements _type _charge _rawdamage) (Utilities|Struct|BreakDamageInformation damageInformation))
  (bind _returnvalue (Class|Tools|CalculateFinalDamage self _elements _rawdamage))
  (Development|PrintString (Utilities|String|ToString(Float) _returnvalue) true true "(R=0.000000,G=0.660000,B=1.000000,A=1.000000)" 1e+02)
  (return true))

(fn Shock
  (return false))