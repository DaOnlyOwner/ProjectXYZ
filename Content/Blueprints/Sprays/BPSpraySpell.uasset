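; Spray spell actor that damages and, for water sprays, pushes whatever is in a cone cast from its origin player.
; Each tick it caches the hits of a cone overlap and, if the damage elements include Water, sends them push messages along the actor's forward vector.
; A looping timer sends damage messages to the cached hits at a set interval and is cleared when the actor is destroyed.
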(event Custom|DamageTick
  (for _array_element (Variables|Default|GetcachedHitResults)
    (Class|DamageAble|ReceiveDamage(Message) _array_element (Variables|Default|GetdamageInformation))))

(event EventBeginPlay
  (bind _returnvalue (Utilities|Time|SetTimerbyEvent (delegate Custom|DamageTick) (Variables|Default|GetInterval) true)))

(event EventDestroyed
  (Utilities|Time|ClearandInvalidateTimerbyHandle (stale EventBeginPlay _returnvalue)))

(event EventTick
  (params (DeltaSeconds :type Float%20%28single-precision%29))
  (bind _outhitresults (Class|Tools|OverlapCone (Variables|Default|GetoriginPlayer self) "ECC_GameTraceChannel1" 3e+01 2e+02 (Utilities|Array|MakeArray 0) true false))
  (bind _output_get (Variables|Default|SetcachedHitResults _outhitresults))
  (if (Utilities|Array|ContainsItem (.Elements (Utilities|Struct|BreakDamageInformation (Variables|Default|GetdamageInformation))) "Water")
    (for _array_element _output_get
      (Class|DamageAble|Push(Message) _array_element (Transformation|GetActorForwardVector)))))

(fn ConstructionScript)